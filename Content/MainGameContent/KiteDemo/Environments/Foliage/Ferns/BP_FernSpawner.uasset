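; BP_FernSpawner is a placeable foliage actor that scatters fern meshes inside an adjustable box, with all event graph events left unused.
; Its construction script sizes SpawnBox from BoxSize, then adds SpawnAmmount static mesh components, each using a random pick from the first three Ferns entries.
; Placement uses random XY within the box, slight height jitter, random yaw and fixed scale, with no seed or ground trace, so layouts reshuffle on reconstruction.
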(event EventBeginPlay)

(event Collision|EventActorBeginOverlap
  (params (OtherActor :type Actor%20Object%20Reference)))

(event EventTick
  (params (DeltaSeconds :type Float%20%28single-precision%29)))

(fn ConstructionScript
  (bind _spawnbox (Variables|Default|GetSpawnBox))
  (bind _boxextent (Variables|/Script/Engine.BoxComponent|GetBoxExtent _spawnbox))
  (bind _relativelocation (Variables|/Script/Engine.SceneComponent|GetRelativeLocation _spawnbox))
  (bind _returnvalue (Math|Random|RandomPointinBoundingBox _relativelocation _boxextent))
  (Components|Box|SetBoxExtent (Variables|Default|GetSpawnBox) (Variables|Default|GetBoxSize) true)
  (for _index (range 1 (Variables|Default|GetSpawnAmmount))
    (bind _returnvalue_2 (AddComponent|AddStaticMeshComponent false (Math|Transform|MakeTransform (Math|Vector|MakeVector (.x _returnvalue) (.y _returnvalue) (Math|Random|RandomFloatinRange 0.0 2e+01)) (Math|Rotator|MakeRotator 0.0 0.0 (Math|Random|RandomFloatinRange 0.0 3.6e+02)) "3.000000,3.000000,3.000000")))
    (Components|StaticMesh|SetStaticMesh _returnvalue_2 (Utilities|Array|Get(acopy) (Variables|Default|GetFerns) (Math|Random|RandomIntegerinRange 0 2)))))