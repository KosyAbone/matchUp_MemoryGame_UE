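; BP_DecorCard is a decorative card for the memory game, built from a block mesh, a front sprite and a backside sprite.
; Its construction script sets the backside sprite image from a back-sprite struct.
; It then checks the current level name, giving both sprites the struct's low-end or high-end material instance.
; The block mesh gets an emissive color material on MemoryLowEndMap and a base color material elsewhere.
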(fn ConstructionScript
  (bind _backside_sprite (Variables|Default|Getbackside_Sprite))
  (bind _backspritestruct (Variables|Default|GetBackSpriteStruct))
  (bind (_paperspriteobject _highendmaterialinstance _lowendmaterialinstance) (Utilities|Struct|BreakBackSpriteStruct _backspritestruct))
  (bind _returnvalue (Game|GetCurrentLevelName true))
  (Rendering|Components|Sprite|SetSprite _backside_sprite _paperspriteobject)
  (Rendering|Material|SetMaterial _backside_sprite 0 (select (Utilities|Enum|Equal(Enum) _returnvalue "MemoryLowEndMap") _lowendmaterialinstance _highendmaterialinstance))
  (Rendering|Material|SetMaterial (Variables|Default|GetBlockMesh) 0 (select (Utilities|Enum|Equal(Enum) _returnvalue "MemoryLowEndMap") "/Game/MainGameContent/MeshAndMaterials/Materials/M_CardsEmissiveColor.M_CardsEmissiveColor" "/Game/MainGameContent/MeshAndMaterials/Materials/M_CardsBaseColor.M_CardsBaseColor")))