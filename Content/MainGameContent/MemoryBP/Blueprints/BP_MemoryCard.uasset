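; Clickable card actor for a memory pairs game, coordinated by its owning MemoryController.
; Timelines animate dealing from the spawn point, flipping on click or touch and reversing out on removal; the last card removed triggers a respawn.
; Flipped cards report to the controller for comparison and display floating score or penalty text, with pair particles and sound.
; Construction picks low-end or high-end materials by level name, and face sprites hide when face down for mobile performance.
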(event OnInputTouchBegin(backside_Sprite)
  (params (FingerIndex :type ETouchIndex%20Enum :default "Touch1") (TouchedComponent :type Primitive%20Component%20Object%20Reference))
  (bind _self self)
  (bind _returnvalue (Transformation|GetActorLocation _self))
  ;[1 1 1] Handle block being clicked
  ;;[1 1 1] Block if CardFace up (Antispam
  (if (== (Components|Timeline|GetPlaybackPosition (Variables|Default|GetFlipAnimation)) 0.0)
    ;;[1 1 1] Only when Controller allows it. DO NOT combine Branches (Antispam and wait for Reverse Event called by controller if Pairs mismatch )
    (if (not (Variables|/Game/MainGameContent/MemoryBP/Blueprints/BP_MemoryController.BP_MemoryController_C|GetBlock (Variables|Default|GetOwningMemoryController)))
      (if (not (Variables|Default|GetIsActive))
        ;;[1 1 1] (Mobile Optimization)
        (Rendering|SetVisibility (Variables|Default|GetSprite) true false)
        (Variables|Default|SetIsActive true)
        (Utilities|FlowControl|Sequence
          (:then_0
            ;;[1 1 1] Add & Compair Event
            (Default|Add&Compair (Variables|Default|GetOwningMemoryController) self))
          (:then_1
            (bind (_direction _locationz _rotation_y) (Timeline|FlipAnimation Play)
              (:Update
                (Transformation|SetActorLocationAndRotation _self (Math|Vector|MakeVector (.x _returnvalue) (.y _returnvalue) _locationz) (Math|Rotator|MakeRotator 0.0 _rotation_y (Variables|/Game/MainGameContent/MemoryBP/Blueprints/BP_MemoryController.BP_MemoryController_C|GetTiltingDegrees (Variables|Default|GetOwningMemoryController)))))
              (:Finished
                ;[1 1 1] (Mobile Optimization)
                (switch Utilities|FlowControl|Switch|SwitchonETimelineDirection _direction
                  (:Backward
                    (Rendering|SetVisibility (Variables|Default|GetSprite) false false))))))
          (:then_2
            (Audio|PlaySound2D (Variables|/Game/MainGameContent/MemoryBP/Blueprints/BP_MemoryController.BP_MemoryController_C|GetSoundOnClick (Variables|Default|GetOwningMemoryController)) 1.0 1.0 0.0 0 0)))))))

(event OnBeginCursorOver(backside_Sprite)
  (params (TouchedComponent :type Primitive%20Component%20Object%20Reference))
  ;[1 1 1] Cards turn blue when hovered by mouse and back to white if the mouse isn't hovering.
  (Rendering|Material|SetMaterial (Variables|Default|GetBlockMesh) 0 "/Game/MainGameContent/MeshAndMaterials/Materials/MI_CardsHighlight.MI_CardsHighlight"))

(event OnClicked(backside_Sprite)
  (params (TouchedComponent :type Primitive%20Component%20Object%20Reference) (ButtonPressed :type Key%20Structure))
  (bind _self self)
  (bind _returnvalue (Transformation|GetActorLocation _self))
  ;[1 1 1] Handle block being clicked
  ;;[1 1 1] Block if CardFace up (Antispam
  (if (== (Components|Timeline|GetPlaybackPosition (Variables|Default|GetFlipAnimation)) 0.0)
    ;;[1 1 1] Only when Controller allows it. DO NOT combine Branches (Antispam and wait for Reverse Event called by controller if Pairs mismatch )
    (if (not (Variables|/Game/MainGameContent/MemoryBP/Blueprints/BP_MemoryController.BP_MemoryController_C|GetBlock (Variables|Default|GetOwningMemoryController)))
      (if (not (Variables|Default|GetIsActive))
        ;;[1 1 1] (Mobile Optimization)
        (Rendering|SetVisibility (Variables|Default|GetSprite) true false)
        (Variables|Default|SetIsActive true)
        (Utilities|FlowControl|Sequence
          (:then_0
            ;;[1 1 1] Add & Compair Event
            (Default|Add&Compair (Variables|Default|GetOwningMemoryController) self))
          (:then_1
            (bind (_direction _locationz _rotation_y) (Timeline|FlipAnimation Play)
              (:Update
                (Transformation|SetActorLocationAndRotation _self (Math|Vector|MakeVector (.x _returnvalue) (.y _returnvalue) _locationz) (Math|Rotator|MakeRotator 0.0 _rotation_y (Variables|/Game/MainGameContent/MemoryBP/Blueprints/BP_MemoryController.BP_MemoryController_C|GetTiltingDegrees (Variables|Default|GetOwningMemoryController)))))
              (:Finished
                ;[1 1 1] (Mobile Optimization)
                (switch Utilities|FlowControl|Switch|SwitchonETimelineDirection _direction
                  (:Backward
                    (Rendering|SetVisibility (Variables|Default|GetSprite) false false))))))
          (:then_2
            (Audio|PlaySound2D (Variables|/Game/MainGameContent/MemoryBP/Blueprints/BP_MemoryController.BP_MemoryController_C|GetSoundOnClick (Variables|Default|GetOwningMemoryController)) 1.0 1.0 0.0 0 0)))))))

(event OnEndCursorOver(backside_Sprite)
  (params (TouchedComponent :type Primitive%20Component%20Object%20Reference))
  ;[1 1 1] Cards turn blue when hovered by mouse and back to white if the mouse isn't hovering.
  (Rendering|Material|SetMaterial (Variables|Default|GetBlockMesh) 0 (select (Variables|Default|GetLowEndMap) "/Game/MainGameContent/MeshAndMaterials/Materials/M_CardsEmissiveColor.M_CardsEmissiveColor" "/Game/MainGameContent/MeshAndMaterials/Materials/M_CardsBaseColor.M_CardsBaseColor")))

(event Custom|HandleControllerClick
  (bind _self self)
  (bind _returnvalue (Transformation|GetActorLocation _self))
  ;[1 1 1] Handle block being clicked
  ;;[1 1 1] Block if CardFace up (Antispam
  (if (== (Components|Timeline|GetPlaybackPosition (Variables|Default|GetFlipAnimation)) 0.0)
    ;;[1 1 1] Only when Controller allows it. DO NOT combine Branches (Antispam and wait for Reverse Event called by controller if Pairs mismatch )
    (if (not (Variables|/Game/MainGameContent/MemoryBP/Blueprints/BP_MemoryController.BP_MemoryController_C|GetBlock (Variables|Default|GetOwningMemoryController)))
      (if (not (Variables|Default|GetIsActive))
        ;;[1 1 1] (Mobile Optimization)
        (Rendering|SetVisibility (Variables|Default|GetSprite) true false)
        (Variables|Default|SetIsActive true)
        (Utilities|FlowControl|Sequence
          (:then_0
            ;;[1 1 1] Add & Compair Event
            (Default|Add&Compair (Variables|Default|GetOwningMemoryController) self))
          (:then_1
            (bind (_direction _locationz _rotation_y) (Timeline|FlipAnimation Play)
              (:Update
                (Transformation|SetActorLocationAndRotation _self (Math|Vector|MakeVector (.x _returnvalue) (.y _returnvalue) _locationz) (Math|Rotator|MakeRotator 0.0 _rotation_y (Variables|/Game/MainGameContent/MemoryBP/Blueprints/BP_MemoryController.BP_MemoryController_C|GetTiltingDegrees (Variables|Default|GetOwningMemoryController)))))
              (:Finished
                ;[1 1 1] (Mobile Optimization)
                (switch Utilities|FlowControl|Switch|SwitchonETimelineDirection _direction
                  (:Backward
                    (Rendering|SetVisibility (Variables|Default|GetSprite) false false))))))
          (:then_2
            (Audio|PlaySound2D (Variables|/Game/MainGameContent/MemoryBP/Blueprints/BP_MemoryController.BP_MemoryController_C|GetSoundOnClick (Variables|Default|GetOwningMemoryController)) 1.0 1.0 0.0 0 0)))))))

(event Custom|DestroySelf
  (bind _owningmemorycontroller (Variables|Default|GetOwningMemoryController))
  (bind _owningmemorycontroller_2 (Variables|Default|GetOwningMemoryController))
  (bind _tiltingdegrees (Variables|/Game/MainGameContent/MemoryBP/Blueprints/BP_MemoryController.BP_MemoryController_C|GetTiltingDegrees _owningmemorycontroller))
  (bind _memorycardscounter (Variables|/Game/MainGameContent/MemoryBP/Blueprints/BP_MemoryController.BP_MemoryController_C|GetMemoryCardsCounter _owningmemorycontroller_2))
  ;[1 1 1] Move to Location Animation & Reversing "DestroySelf" Event Call
  ;;[1 1 1] Move back to Spawn and destroy after
  (bind _returnvalue (Utilities|Array|RemoveItem _memorycardscounter self))
  (Utilities|FlowControl|Delay 1.75)
  (Utilities|FlowControl|Sequence
    (:then_0
      (bind (_direction _forwardz _reverse_z _forwardlerp _reverselerp) (Timeline|MoveToLocationAnimation Reverse)
        (:Update
          (Transformation|SetActorLocation (Math|Vector|MakeVector (.x (Math|Vector|Lerp(Vector) (Variables|/Game/MainGameContent/MemoryBP/Blueprints/BP_MemoryController.BP_MemoryController_C|GetInitialSpawnLocation (Variables|Default|GetOwningMemoryController)) (Variables|Default|GetMoveToLocation) (select _returnvalue _reverselerp _forwardlerp))) (.y (Math|Vector|Lerp(Vector) (Variables|/Game/MainGameContent/MemoryBP/Blueprints/BP_MemoryController.BP_MemoryController_C|GetInitialSpawnLocation (Variables|Default|GetOwningMemoryController)) (Variables|Default|GetMoveToLocation) (select _returnvalue _reverselerp _forwardlerp))) (select _returnvalue _reverse_z _forwardz)) false false)
          ;[1 1 1] Rotate and compensate Controller's "TiltingDegress" depending on Timelines direction
          (Transformation|SetActorRotation (Utilities|Select :Index _direction :Forward (Math|Rotator|Lerp(Rotator) (Math|Rotator|MakeRotator 1.8e+02 0.0 (+ 1.8e+02 _tiltingdegrees)) (Math|Rotator|MakeRotator 1.8e+02 0.0 (+ -1.8e+02 _tiltingdegrees)) _forwardlerp) :Backward (Math|Rotator|Lerp(Rotator) (Math|Rotator|MakeRotator 1.8e+02 0.0 (+ 1.8e+02 _tiltingdegrees)) (Math|Rotator|MakeRotator 0.0 0.0 (+ 0.0 _tiltingdegrees)) _reverselerp))))
        (:Finished
          ;[1 1 1] Enable Collision response only when Card on Table
          (Collision|SetCollisionResponsetoChannel (Variables|Default|Getbackside_Sprite) "ECC_Visibility" "ECR_Block"))))
    (:then_1
      (if (== (Utilities|Array|Length _memorycardscounter) 0)
        (Default|RespawnCards _owningmemorycontroller_2)))
    (:then_2
      (Utilities|FlowControl|Delay 1.0)
      (Actor|DestroyActor self))))

(event Custom|Reverse
  (bind _self self)
  (bind _returnvalue (Transformation|GetActorLocation _self))
  ;[1 1 1] Handle block being clicked
  (Utilities|FlowControl|Delay 1.0)
  (bind (_direction _locationz _rotation_y) (Timeline|FlipAnimation ReverseFromEnd)
    (:Update
      (Transformation|SetActorLocationAndRotation _self (Math|Vector|MakeVector (.x _returnvalue) (.y _returnvalue) _locationz) (Math|Rotator|MakeRotator 0.0 _rotation_y (Variables|/Game/MainGameContent/MemoryBP/Blueprints/BP_MemoryController.BP_MemoryController_C|GetTiltingDegrees (Variables|Default|GetOwningMemoryController)))))
    (:Finished
      ;[1 1 1] (Mobile Optimization)
      (switch Utilities|FlowControl|Switch|SwitchonETimelineDirection _direction
        (:Backward
          (Rendering|SetVisibility (Variables|Default|GetSprite) false false))))))

(event Custom|DisplayScoreOnCard%20B
  (bind _owningmemorycontroller (Variables|Default|GetOwningMemoryController))
  (bind _owningmemorycontroller_2 (Variables|Default|GetOwningMemoryController))
  (bind _b_card (Variables|/Game/MainGameContent/MemoryBP/Blueprints/BP_MemoryController.BP_MemoryController_C|GetB%20Card _owningmemorycontroller))
  (bind _penalty (Variables|/Game/MainGameContent/MemoryBP/Blueprints/BP_MemoryController.BP_MemoryController_C|GetPenalty _owningmemorycontroller_2))
  (bind _pairsparticle (Variables|/Game/MainGameContent/MemoryBP/Blueprints/BP_MemoryController.BP_MemoryController_C|GetPairsParticle _owningmemorycontroller))
  (bind _a_card (Variables|/Game/MainGameContent/MemoryBP/Blueprints/BP_MemoryController.BP_MemoryController_C|GetA%20Card _owningmemorycontroller))
  (bind _returnvalue (Transformation|GetActorLocation _b_card))
  (bind _returnvalue_2 (Transformation|GetActorLocation _a_card))
  ;[1 1 1] Add SoundFX, Score and Particle Logic
  ;;[1 1 1] Add Particles if user provieds them on the "MemoryController"
  (Variables|Default|SetIsMinus? false)
  (Utilities|IsValid _pairsparticle ; Did user select any Particle?
    (:Is%20Valid
      (Utilities|FlowControl|Sequence
        (:then_0
          (bind _returnvalue_3 (Effects|SpawnEmitteratLocation _pairsparticle (Math|Vector|MakeVector (.x _returnvalue_2) (.y _returnvalue_2) 5e+01) "0, 0, 0" "1.000000,1.000000,1.000000" false))
          (bind _returnvalue_4 (Effects|SpawnEmitteratLocation _pairsparticle (Math|Vector|MakeVector (.x _returnvalue) (.y _returnvalue) 5e+01) "0, 0, 0" "1.000000,1.000000,1.000000" false))
          (Components|Activation|SetActive _returnvalue_4 false false)
          ;;[1 1 1] Draw Text on Cards
          (Utilities|FlowControl|Delay 0.5 :!label _label)
          (bind _returnvalue_5 (AddComponent|AddTextRenderComponent true (Math|Transform|MakeTransform (Math|Vector|MakeVector (+ (.x _returnvalue) 1e+02) (- (.y _returnvalue) 2e+01) 2e+02) "90.000000,-90.000000,0.000000" "1.000000,1.000000,1.000000")))
          (Transformation|AttachComponentToComponent _returnvalue_5 0 "None" "KeepWorld" "KeepWorld" "KeepWorld" true)
          (Rendering|Components|TextRender|SetText _returnvalue_5 (select (Variables|Default|GetIsMinus?) (select (== _penalty 0) "" (Utilities|Text|FormatText "-{Penalty}" _penalty)) (Utilities|Text|FormatText "+{Combo}" (* (- (Variables|/Game/MainGameContent/MemoryBP/Blueprints/BP_MemoryController.BP_MemoryController_C|GetMultiCache%20%28DoNOTUse%29 _owningmemorycontroller_2) 1) (Variables|/Game/MainGameContent/MemoryBP/Blueprints/BP_MemoryController.BP_MemoryController_C|GetPairsPointsValue _owningmemorycontroller_2)))))
          (Rendering|Components|TextRender|SetTextRenderColor _returnvalue_5 (select (Variables|Default|GetIsMinus?) (Math|Color|MakeColor 0 0 255) (Math|Color|MakeColor 0 255 0)))
          ;;;[1 1 1] Animate Text
          (bind _textfloatz (Timeline|FloatText PlayFromStart)
            (:Update
              (Transformation|AddLocalOffset _returnvalue_5 (Math|Vector|MakeVector 0.0 0.0 _textfloatz) false false))
            (:Finished
              (Components|DestroyComponent _returnvalue_5))))
        (:then_1
          (Utilities|FlowControl|Delay 0.5)
          (Components|Activation|SetActive _returnvalue_4 true false)
          (Utilities|FlowControl|DoOnce false :!label _label_2
            (:Completed
              ;;[1 1 1] Play "Pair Sound Cue" if provided
              (Audio|PlaySound2D (Variables|/Game/MainGameContent/MemoryBP/Blueprints/BP_MemoryController.BP_MemoryController_C|GetPairsSoundCue (Variables|Default|GetOwningMemoryController)) 1.0 1.0 0.0 0 0))))))
    (:Is%20Not%20Valid
      (Utilities|FlowControl|Sequence
        (:then_0
          (goto _label))
        (:then_1
          (Utilities|FlowControl|Delay 0.2)
          (goto _label_2))))))

(event Custom|DisplayMinusOnCardB
  (bind _owningmemorycontroller (Variables|Default|GetOwningMemoryController))
  (bind _owningmemorycontroller_2 (Variables|Default|GetOwningMemoryController))
  (bind _b_card (Variables|/Game/MainGameContent/MemoryBP/Blueprints/BP_MemoryController.BP_MemoryController_C|GetB%20Card _owningmemorycontroller))
  (bind _penalty (Variables|/Game/MainGameContent/MemoryBP/Blueprints/BP_MemoryController.BP_MemoryController_C|GetPenalty _owningmemorycontroller_2))
  (bind _returnvalue (Transformation|GetActorLocation _b_card))
  ;[1 1 1] Add SoundFX, Score and Particle Logic
  ;;[1 1 1] Draw Minus Points on second clicked card. Don't do it if we have 0 Points.
  (Variables|Default|SetIsMinus? true)
  (if (not (== (Variables|/Game/MainGameContent/MemoryBP/Blueprints/BP_MemoryController.BP_MemoryController_C|GetScoreCache%20%28DoNOTUse%29 (Variables|Default|GetOwningMemoryController)) 0))
    ;;[1 1 1] Draw Text on Cards
    (Utilities|FlowControl|Delay 0.5)
    (bind _returnvalue_2 (AddComponent|AddTextRenderComponent true (Math|Transform|MakeTransform (Math|Vector|MakeVector (+ (.x _returnvalue) 1e+02) (- (.y _returnvalue) 2e+01) 2e+02) "90.000000,-90.000000,0.000000" "1.000000,1.000000,1.000000")))
    (Transformation|AttachComponentToComponent _returnvalue_2 0 "None" "KeepWorld" "KeepWorld" "KeepWorld" true)
    (Rendering|Components|TextRender|SetText _returnvalue_2 (select (Variables|Default|GetIsMinus?) (select (== _penalty 0) "" (Utilities|Text|FormatText "-{Penalty}" _penalty)) (Utilities|Text|FormatText "+{Combo}" (* (- (Variables|/Game/MainGameContent/MemoryBP/Blueprints/BP_MemoryController.BP_MemoryController_C|GetMultiCache%20%28DoNOTUse%29 _owningmemorycontroller_2) 1) (Variables|/Game/MainGameContent/MemoryBP/Blueprints/BP_MemoryController.BP_MemoryController_C|GetPairsPointsValue _owningmemorycontroller_2)))))
    (Rendering|Components|TextRender|SetTextRenderColor _returnvalue_2 (select (Variables|Default|GetIsMinus?) (Math|Color|MakeColor 0 0 255) (Math|Color|MakeColor 0 255 0)))
    ;;;[1 1 1] Animate Text
    (bind _textfloatz (Timeline|FloatText PlayFromStart)
      (:Update
        (Transformation|AddLocalOffset _returnvalue_2 (Math|Vector|MakeVector 0.0 0.0 _textfloatz) false false))
      (:Finished
        (Components|DestroyComponent _returnvalue_2)))))

(event EventBeginPlay
  (bind _owningmemorycontroller (Variables|Default|GetOwningMemoryController))
  (bind _tiltingdegrees (Variables|/Game/MainGameContent/MemoryBP/Blueprints/BP_MemoryController.BP_MemoryController_C|GetTiltingDegrees _owningmemorycontroller))
  ;[1 1 1] Move to Location Animation & Reversing "DestroySelf" Event Call
  ;;[1 0 0] Begin Play
  (Utilities|FlowControl|Delay 0.5)
  (bind (_direction _forwardz _reverse_z _forwardlerp _reverselerp) (Timeline|MoveToLocationAnimation PlayFromStart)
    (:Update
      (Transformation|SetActorLocation (Math|Vector|MakeVector (.x (Math|Vector|Lerp(Vector) (Variables|/Game/MainGameContent/MemoryBP/Blueprints/BP_MemoryController.BP_MemoryController_C|GetInitialSpawnLocation (Variables|Default|GetOwningMemoryController)) (Variables|Default|GetMoveToLocation) (select (stale Custom|DestroySelf _returnvalue) _reverselerp _forwardlerp))) (.y (Math|Vector|Lerp(Vector) (Variables|/Game/MainGameContent/MemoryBP/Blueprints/BP_MemoryController.BP_MemoryController_C|GetInitialSpawnLocation (Variables|Default|GetOwningMemoryController)) (Variables|Default|GetMoveToLocation) (select (stale Custom|DestroySelf _returnvalue) _reverselerp _forwardlerp))) (select (stale Custom|DestroySelf _returnvalue) _reverse_z _forwardz)) false false)
      ;[1 1 1] Rotate and compensate Controller's "TiltingDegress" depending on Timelines direction
      (Transformation|SetActorRotation (Utilities|Select :Index _direction :Forward (Math|Rotator|Lerp(Rotator) (Math|Rotator|MakeRotator 1.8e+02 0.0 (+ 1.8e+02 _tiltingdegrees)) (Math|Rotator|MakeRotator 1.8e+02 0.0 (+ -1.8e+02 _tiltingdegrees)) _forwardlerp) :Backward (Math|Rotator|Lerp(Rotator) (Math|Rotator|MakeRotator 1.8e+02 0.0 (+ 1.8e+02 _tiltingdegrees)) (Math|Rotator|MakeRotator 0.0 0.0 (+ 0.0 _tiltingdegrees)) _reverselerp))))
    (:Finished
      ;[1 1 1] Enable Collision response only when Card on Table
      (Collision|SetCollisionResponsetoChannel (Variables|Default|Getbackside_Sprite) "ECC_Visibility" "ECR_Block"))))

(event EventActorOnInputTouchBegin
  (params (FingerIndex :type ETouchIndex%20Enum :default "Touch1"))
  (bind _self self)
  (bind _returnvalue (Transformation|GetActorLocation _self))
  ;[1 1 1] Handle block being clicked
  ;;[1 1 1] Block if CardFace up (Antispam
  (if (== (Components|Timeline|GetPlaybackPosition (Variables|Default|GetFlipAnimation)) 0.0)
    ;;[1 1 1] Only when Controller allows it. DO NOT combine Branches (Antispam and wait for Reverse Event called by controller if Pairs mismatch )
    (if (not (Variables|/Game/MainGameContent/MemoryBP/Blueprints/BP_MemoryController.BP_MemoryController_C|GetBlock (Variables|Default|GetOwningMemoryController)))
      (if (not (Variables|Default|GetIsActive))
        ;;[1 1 1] (Mobile Optimization)
        (Rendering|SetVisibility (Variables|Default|GetSprite) true false)
        (Variables|Default|SetIsActive true)
        (Utilities|FlowControl|Sequence
          (:then_0
            ;;[1 1 1] Add & Compair Event
            (Default|Add&Compair (Variables|Default|GetOwningMemoryController) self))
          (:then_1
            (bind (_direction _locationz _rotation_y) (Timeline|FlipAnimation Play)
              (:Update
                (Transformation|SetActorLocationAndRotation _self (Math|Vector|MakeVector (.x _returnvalue) (.y _returnvalue) _locationz) (Math|Rotator|MakeRotator 0.0 _rotation_y (Variables|/Game/MainGameContent/MemoryBP/Blueprints/BP_MemoryController.BP_MemoryController_C|GetTiltingDegrees (Variables|Default|GetOwningMemoryController)))))
              (:Finished
                ;[1 1 1] (Mobile Optimization)
                (switch Utilities|FlowControl|Switch|SwitchonETimelineDirection _direction
                  (:Backward
                    (Rendering|SetVisibility (Variables|Default|GetSprite) false false))))))
          (:then_2
            (Audio|PlaySound2D (Variables|/Game/MainGameContent/MemoryBP/Blueprints/BP_MemoryController.BP_MemoryController_C|GetSoundOnClick (Variables|Default|GetOwningMemoryController)) 1.0 1.0 0.0 0 0)))))))

(fn ConstructionScript
  (bind _backside_sprite (Variables|Default|Getbackside_Sprite))
  (bind _backspritestruct (Variables|Default|GetBackSpriteStruct))
  (bind (_paperspriteobject _highendmaterialinstance _lowendmaterialinstance) (Utilities|Struct|BreakBackSpriteStruct _backspritestruct))
  (bind _returnvalue (Game|GetCurrentLevelName true))
  (Rendering|Components|Sprite|SetSprite _backside_sprite _paperspriteobject)
  (Rendering|Material|SetMaterial _backside_sprite 0 (select (Utilities|Enum|Equal(Enum) _returnvalue "MemoryLowEndMap") _lowendmaterialinstance _highendmaterialinstance))
  (Rendering|Material|SetMaterial (Variables|Default|GetBlockMesh) 0 (select (Utilities|Enum|Equal(Enum) _returnvalue "MemoryLowEndMap") "/Game/MainGameContent/MeshAndMaterials/Materials/M_CardsEmissiveColor.M_CardsEmissiveColor" "/Game/MainGameContent/MeshAndMaterials/Materials/M_CardsBaseColor.M_CardsBaseColor"))
  (Variables|Default|SetLowEndMap (Utilities|Enum|Equal(Enum) _returnvalue "MemoryLowEndMap")))