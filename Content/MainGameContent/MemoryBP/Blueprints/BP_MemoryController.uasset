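; Controller for a pair-matching memory card game that runs rounds, scoring and the score banner HUD.
; Construction builds a spawn-slot grid, where duplicated random sprites become card actors spawned with a delayed-loop macro.
; Cards report clicks to Add&Compair, which alternates A/B picks by FlipFlop, then rewards combo matches or penalizes mismatches.
; RespawnCards scales pair points, grows the deck every other level and saves progress, which BeginPlay reloads.
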(event Custom|Add%20&Compair
  (params (SelfRefMemoryCard :type Actor%20Object%20Reference))
  (bind _returnvalue (Actor|GetComponentbyClass SelfRefMemoryCard "/Script/Paper2D.PaperSpriteComponent"))
  (bind _sourcesprite (Variables|/Script/Paper2D.PaperSpriteComponent|GetSourceSprite _returnvalue))
  ;[1 1 1] Core "Memory" like Gameplay Logic! Its fired when clicking on a card (Event Call inside BP_MemoryCard)
  ;;[1 1 1] Check if cards identical on two consecutive clicks
  (bind _isa (Utilities|FlowControl|FlipFlop)
    (:A
      (Variables|Default|SetA%20Card SelfRefMemoryCard)
      (bind _output_get (Variables|Default|SetA%20CardSprite _sourcesprite)))
    (:B
      (Variables|Default|SetB%20Card SelfRefMemoryCard)
      (bind _output_get_2 (Variables|Default|SetB%20CardSprite _sourcesprite))))
  (if (== _output_get _output_get_2)
    (Utilities|FlowControl|Sequence
      (:then_0
        ;;[1 1 1] Cards Identical Logic
        (bind _asbp_memory_card (Utilities|Casting|CastToBP_MemoryCard (Variables|Default|GetA%20Card)))
        (Default|DestroySelf _asbp_memory_card)
        ;;;[0.04706 1 0] Add Score on Card
        (Default|DisplayScoreonCardB _asbp_memory_card))
      (:then_1
        (bind _asbp_memory_card_2 (Utilities|Casting|CastToBP_MemoryCard (Variables|Default|GetB%20Card)))
        (Default|DestroySelf _asbp_memory_card_2)
        ;;;[0.04706 1 0] Delete Cards Reference
        (Variables|Default|SetA%20CardSprite 0)
        (Variables|Default|SetB%20CardSprite 0)
        ;;;[0.04706 1 0] Calculate Score Add Combo
        (Variables|Default|SetScoreCache%20%28DoNOTUse%29 (+ (* (Variables|Default|GetMultiCache%20%28DoNOTUse%29) (Variables|MemorySettings|GetPairsPointsValue)) (Variables|Default|GetScoreCache%20%28DoNOTUse%29)))
        (Variables|Default|SetMultiCache%20%28DoNOTUse%29 (+ (Variables|Default|GetMultiCache%20%28DoNOTUse%29) 1))
        ;;;[0.04706 1 0] Wait and set real values to use and display on UMG
        (Utilities|FlowControl|Delay 1.0)
        (bind _output_get_3 (Variables|Default|SetScore (Variables|Default|GetScoreCache%20%28DoNOTUse%29)))
        (bind _output_get_4 (Variables|Default|SetMultiplicator (- (Variables|Default|GetMultiCache%20%28DoNOTUse%29) 1)))
        (Rendering|Components|TextRender|SetText (Variables|/Game/MainGameContent/MemoryBP/Blueprints/UMG/UI_ScoreBanner.UI_ScoreBanner_C|GetCombo (Variables|Default|GetScoreBannerRef)) (Utilities|Text|ToText(Integer) _output_get_4))
        (Rendering|Components|TextRender|SetText (Variables|/Game/MainGameContent/MemoryBP/Blueprints/UMG/UI_ScoreBanner.UI_ScoreBanner_C|GetScorePoints (Variables|Default|GetScoreBannerRef)) (Utilities|Text|ToText(Integer) _output_get_3))))
    (elif (not _isa)
      ;;[1 1 1] Cards mismatching Logic
      (Variables|Default|SetBlock true) ; Used by BP_MemoryCard
      (Utilities|FlowControl|Delay 0.2)
      ;;;[1 0.01961 0] "Reverse" targeting the Memory Cards will turn them face down again
      (Variables|Default|SetBlock false) ; Used by BP_MemoryCard
      (bind _asbp_memory_card_3 (Utilities|Casting|CastToBP_MemoryCard (Variables|Default|GetA%20Card)))
      (Default|Reverse _asbp_memory_card_3)
      (Variables|/Game/MainGameContent/MemoryBP/Blueprints/BP_MemoryCard.BP_MemoryCard_C|SetIsActive _asbp_memory_card_3 false)
      (bind _asbp_memory_card_4 (Utilities|Casting|CastToBP_MemoryCard (Variables|Default|GetB%20Card)))
      (Default|Reverse _asbp_memory_card_4)
      ;;;[1 0.01961 0] Display minus points on Cards, set references and reset Cards
      (Default|DisplayMinusonCardB _asbp_memory_card_4)
      (Variables|/Game/MainGameContent/MemoryBP/Blueprints/BP_MemoryCard.BP_MemoryCard_C|SetIsActive _asbp_memory_card_4 false)
      (Variables|Default|SetA%20CardSprite 0)
      (Variables|Default|SetB%20CardSprite 0)
      ;;;[1 0.01961 0] Reset Combo
      (Variables|Default|SetMultiCache%20%28DoNOTUse%29 1)
      ;;;[1 0.01961 0] Substract "Penalty if any other than 0
      (Variables|Default|SetScoreCache%20%28DoNOTUse%29 (Math|Integer|Clamp(Integer) (- (Variables|Default|GetScoreCache%20%28DoNOTUse%29) (Variables|MemorySettings|GetPenalty)) 0 (Variables|Default|GetScoreCache%20%28DoNOTUse%29)))
      ;;;[1 0.01961 0] Wait and set real values to use and display on UMG
      (Utilities|FlowControl|Delay 1.0)
      (Variables|Default|SetMultiplicator 0)
      (bind _output_get_5 (Variables|Default|SetScore (Variables|Default|GetScoreCache%20%28DoNOTUse%29)))
      (Variables|Default|SetScoreCache%20%28DoNOTUse%29 _output_get_5)
      (Rendering|Components|TextRender|SetText (Variables|/Game/MainGameContent/MemoryBP/Blueprints/UMG/UI_ScoreBanner.UI_ScoreBanner_C|GetScorePoints (Variables|Default|GetScoreBannerRef)) (Utilities|Text|ToText(Integer) _output_get_5))
      (Rendering|Components|TextRender|SetText (Variables|/Game/MainGameContent/MemoryBP/Blueprints/UMG/UI_ScoreBanner.UI_ScoreBanner_C|GetCombo (Variables|Default|GetScoreBannerRef)) "0"))))

(event Custom|SaveGame
  ;[0 0.5572 1] SaveLogic
  ;;[1 1 1] Create or overwrite SaveGame
  (Development|PrintString "SAVED")
  (bind _returnvalue (SaveGame|CreateSaveGameObject "/Game/MainGameContent/MemoryBP/SaveGame/BP_SaveGameSlot.BP_SaveGameSlot_C"))
  (bind _output_get (Variables|Default|SetSaveGameRef _returnvalue))
  (Variables|/Game/MainGameContent/MemoryBP/SaveGame/BP_SaveGameSlot.BP_SaveGameSlot_C|SetLevelSave _output_get (Variables|Default|GetLevel))
  (Variables|/Game/MainGameContent/MemoryBP/SaveGame/BP_SaveGameSlot.BP_SaveGameSlot_C|SetScoreSave _output_get (Variables|Default|GetScoreCache%20%28DoNOTUse%29))
  (Variables|/Game/MainGameContent/MemoryBP/SaveGame/BP_SaveGameSlot.BP_SaveGameSlot_C|SetMultiplicatorSave _output_get (Variables|Default|GetMultiplicator))
  (Variables|/Game/MainGameContent/MemoryBP/SaveGame/BP_SaveGameSlot.BP_SaveGameSlot_C|SetMemorySizeSave _output_get (Variables|MemorySettings|GetMemorySize))
  (Variables|/Game/MainGameContent/MemoryBP/SaveGame/BP_SaveGameSlot.BP_SaveGameSlot_C|SetPairPointsSave _output_get (Variables|MemorySettings|GetPairsPointsValue))
  (SaveGame|SaveGametoSlot _output_get "FirstSlot"))

(event Custom|RespawnCards
  (bind _cardsspawnpool (Variables|Default|GetCardsSpawnPool))
  (bind _cardsspawnpool_2 (Variables|Default|GetCardsSpawnPool))
  (bind _spawnlocationspool (Variables|Default|GetSpawnLocationsPool))
  (bind _pairpointsvaluecache_donotuse_ (Variables|Default|GetPairPointsValueCache%28DoNotUse%29))
  (bind _cardsspawnpoolcache (Variables|Default|GetCardsSpawnPoolCache))
  ;[1 0 0] RespawnCards Event! Gets called by "BP_MemoryCard" when the "MemoryCardsCounter" array owned by this controller reaches 0
  ;[1 1 1] Add 2 additional Cards to spawn after beating 2 Levels in a row using a FlipFlop
  (Utilities|FlowControl|Delay 2.0)
  (bind _isa (Utilities|FlowControl|FlipFlop) ; Add +2 on second round
    (:A
      _)
    (:B
      _))
  (Variables|MemorySettings|SetPairsPointsValue (+ (/ (* (+ (Variables|Default|GetLevel) 1) _pairpointsvaluecache_donotuse_) 10) _pairpointsvaluecache_donotuse_))
  (Variables|MemorySettings|SetMemorySize (+ (Variables|MemorySettings|GetMemorySize) (select _isa 0 2)))
  ;[1 1 1] Random Spawn Points on each Round
  (Utilities|Array|Clear (Variables|Default|GetSpawnLocationsPool))
  (for _array_element (Variables|Default|GetSpawnSlots)
    (Utilities|Array|AddUnique (Variables|Default|GetSpawnLocationsPool) _array_element))
  (Utilities|FlowControl|Sequence
    (:then_0
      ;[1 1 1] Add +1 to Level Counter...
      (Utilities|FlowControl|Delay 0.6)
      (bind _result (Math|Integer|IncrementInt (Variables|Default|GetLevel))
        (:%20%20
          ;[1 1 1] ...and display value in UMG
          (Rendering|Components|TextRender|SetText (Variables|/Game/MainGameContent/MemoryBP/Blueprints/UMG/UI_ScoreBanner.UI_ScoreBanner_C|GetLevelNumber (Variables|Default|GetScoreBannerRef)) (Utilities|Text|ToText(Integer) _result))
          ;[0 0.5569 1] SaveGame each round
          (CallFunction|SaveGame))))
    (:then_1
      ;[1 1 1] Spawn Cards
      ;;[1 1 1] Logic making sure there are always 2 identical cards
      (for _index (range 0 (Math|Integer|Clamp(Integer) (- (Variables|MemorySettings|GetMemorySize) 1) 3 69))
        (Utilities|FlowControl|FlipFlop
          (:A
            (bind _output_get (Variables|Default|SetDuplicateSprite (Utilities|Array|Get(acopy) _cardsspawnpool (Math|Random|RandomIntegerinRange 0 (- (Utilities|Array|Length (Variables|Default|GetCardsSpawnPool)) 1))))))
          (:B
            (Utilities|Array|RemoveItem _cardsspawnpool _output_get)))
        (Utilities|Array|Add (Variables|Default|GetCardsSpawnPoolCache) _output_get))
      (Utilities|FlowControl|Delay 0.5) ; Needs Delay for accurate Loop with Delay on first Startup
      ;;[1 1 1] Do "MemorySize" ammount of times
      (Utilities|ForLoopwithDelay 0.2 0 (Math|Integer|Clamp(Integer) (- (Variables|MemorySettings|GetMemorySize) 1) 3 69)
        (:LoopBody
          (bind _returnvalue (Game|SpawnActorfromClass "/Game/MainGameContent/MemoryBP/Blueprints/BP_MemoryCard.BP_MemoryCard_C" (Math|Transform|MakeTransform (Variables|MemorySettings|GetInitialSpawnLocation) (Math|Rotator|MakeRotator 0.0 1.8e+02 (Variables|MemorySettings|GetTiltingDegrees)) "0.900000,0.900000,0.900000") "AlwaysSpawn" "OverrideRootScale" 0 self 0)) ; Spawn a Card
          (bind _output_get_2 (Variables|/Game/MainGameContent/MemoryBP/Blueprints/BP_MemoryCard.BP_MemoryCard_C|SetMoveToLocation _returnvalue (Utilities|Array|Get(acopy) _spawnlocationspool (Math|Random|RandomIntegerinRange 0 (- (Utilities|Array|Length _spawnlocationspool) 1)))))
          (Utilities|Array|Add (Variables|Default|GetMemoryCardsCounter) _returnvalue)
          (Utilities|Array|RemoveItem (Variables|Default|GetSpawnLocationsPool) _output_get_2) ; Remove because occupied
          (bind _output_get_3 (Variables|Default|SetCachedIndex (Math|Random|RandomIntegerinRange 0 (- (Utilities|Array|Length _cardsspawnpoolcache) 1))))
          (bind _output_get_4 (Variables|Default|SetCachedSprite (Utilities|Array|Get(acopy) _cardsspawnpoolcache _output_get_3)))
          (Rendering|Components|Sprite|SetSprite (Variables|/Game/MainGameContent/MemoryBP/Blueprints/BP_MemoryCard.BP_MemoryCard_C|GetSprite _returnvalue) _output_get_4)
          (Utilities|Array|RemoveIndex (Variables|Default|GetCardsSpawnPoolCache) _output_get_3) ; DO NOT USE "REMOVE ITEM"\n(That would remove ALL instances\nof said item, deleting the duplicate\nMemoryCard too!)
          ;;[1 1 1] Refill "CardsSpawnPool" only when its Empty
          (if (== (Utilities|Array|Length _cardsspawnpool_2) 0)
            (for _array_element_2 (Utilities|Struct|BreakFrontSpriteStruct (Variables|Default|GetFrontSpriteStruct))
              (Utilities|Array|AddUnique _cardsspawnpool_2 _array_element_2))))))))

(event Custom|LoadSave
  ;[0 0.5572 1] SaveLogic
  ;;[1 1 1] Only if savegame exists
  (bind _returnvalue (SaveGame|DoesSaveGameExist "FirstSlot"))
  (if _returnvalue
    ;;[1 1 1] Load SaveGame
    (bind _returnvalue_2 (SaveGame|LoadGamefromSlot "FirstSlot"))
    (bind _asbp_save_game_slot (Utilities|Casting|CastToBP_SaveGameSlot _returnvalue_2))
    (Variables|Default|SetLevel (Variables|/Game/MainGameContent/MemoryBP/SaveGame/BP_SaveGameSlot.BP_SaveGameSlot_C|GetLevelSave _asbp_save_game_slot))
    (bind _output_get (Variables|Default|SetScoreCache%20%28DoNOTUse%29 (Variables|/Game/MainGameContent/MemoryBP/SaveGame/BP_SaveGameSlot.BP_SaveGameSlot_C|GetScoreSave _asbp_save_game_slot)))
    (Variables|Default|SetScore _output_get)
    (Variables|Default|SetMultiplicator (Variables|/Game/MainGameContent/MemoryBP/SaveGame/BP_SaveGameSlot.BP_SaveGameSlot_C|GetMultiplicatorSave _asbp_save_game_slot))
    (Variables|MemorySettings|SetMemorySize (Variables|/Game/MainGameContent/MemoryBP/SaveGame/BP_SaveGameSlot.BP_SaveGameSlot_C|GetMemorySizeSave _asbp_save_game_slot))
    (Variables|Default|SetPairPointsValueCache%28DoNotUse%29 (Variables|/Game/MainGameContent/MemoryBP/SaveGame/BP_SaveGameSlot.BP_SaveGameSlot_C|GetPairPointsSave _asbp_save_game_slot))
    ;;;[1 0 0.9451] Must Wait to override: (Same BubbleColor)
    (Utilities|FlowControl|Delay 0.1)
    (Variables|MemorySettings|SetPairsPointsValue (Variables|/Game/MainGameContent/MemoryBP/SaveGame/BP_SaveGameSlot.BP_SaveGameSlot_C|GetPairPointsSave _asbp_save_game_slot))))

(event EventBeginPlay
  (bind _cardsspawnpool (Variables|Default|GetCardsSpawnPool))
  (bind _cardsspawnpool_2 (Variables|Default|GetCardsSpawnPool))
  (bind _spawnlocationspool (Variables|Default|GetSpawnLocationsPool))
  (bind _cardsspawnpoolcache (Variables|Default|GetCardsSpawnPoolCache))
  ;[1 0 0] Load previously saved game (with scores) on BeginPlay
  ;;[0 0.5569 1] SaveLogic
  (CallFunction|LoadSave)
  (Utilities|FlowControl|Sequence
    (:then_0
      ;[1 1 1] Add Refs, select Cards and possible Spawn Points
      (Variables|Default|SetPairPointsValueCache%28DoNotUse%29 (Variables|MemorySettings|GetPairsPointsValue))
      (for _array_element (Utilities|Struct|BreakFrontSpriteStruct (Variables|Default|GetFrontSpriteStruct))
        (Utilities|Array|AddUnique (Variables|Default|GetCardsSpawnPool) _array_element))
      (for _array_element_2 (Variables|Default|GetSpawnSlots)
        (Utilities|Array|AddUnique (Variables|Default|GetSpawnLocationsPool) _array_element_2))
      ;[1 1 1] Spawn Cards
      ;;[1 1 1] Logic making sure there are always 2 identical cards
      (for _index (range 0 (Math|Integer|Clamp(Integer) (- (Variables|MemorySettings|GetMemorySize) 1) 3 69))
        (Utilities|FlowControl|FlipFlop
          (:A
            (bind _output_get (Variables|Default|SetDuplicateSprite (Utilities|Array|Get(acopy) _cardsspawnpool (Math|Random|RandomIntegerinRange 0 (- (Utilities|Array|Length (Variables|Default|GetCardsSpawnPool)) 1))))))
          (:B
            (Utilities|Array|RemoveItem _cardsspawnpool _output_get)))
        (Utilities|Array|Add (Variables|Default|GetCardsSpawnPoolCache) _output_get))
      (Utilities|FlowControl|Delay 0.5) ; Needs Delay for accurate Loop with Delay on first Startup
      ;;[1 1 1] Do "MemorySize" ammount of times
      (Utilities|ForLoopwithDelay 0.2 0 (Math|Integer|Clamp(Integer) (- (Variables|MemorySettings|GetMemorySize) 1) 3 69)
        (:LoopBody
          (bind _returnvalue (Game|SpawnActorfromClass "/Game/MainGameContent/MemoryBP/Blueprints/BP_MemoryCard.BP_MemoryCard_C" (Math|Transform|MakeTransform (Variables|MemorySettings|GetInitialSpawnLocation) (Math|Rotator|MakeRotator 0.0 1.8e+02 (Variables|MemorySettings|GetTiltingDegrees)) "0.900000,0.900000,0.900000") "AlwaysSpawn" "OverrideRootScale" 0 self 0)) ; Spawn a Card
          (bind _output_get_2 (Variables|/Game/MainGameContent/MemoryBP/Blueprints/BP_MemoryCard.BP_MemoryCard_C|SetMoveToLocation _returnvalue (Utilities|Array|Get(acopy) _spawnlocationspool (Math|Random|RandomIntegerinRange 0 (- (Utilities|Array|Length _spawnlocationspool) 1)))))
          (Utilities|Array|Add (Variables|Default|GetMemoryCardsCounter) _returnvalue)
          (Utilities|Array|RemoveItem (Variables|Default|GetSpawnLocationsPool) _output_get_2) ; Remove because occupied
          (bind _output_get_3 (Variables|Default|SetCachedIndex (Math|Random|RandomIntegerinRange 0 (- (Utilities|Array|Length _cardsspawnpoolcache) 1))))
          (bind _output_get_4 (Variables|Default|SetCachedSprite (Utilities|Array|Get(acopy) _cardsspawnpoolcache _output_get_3)))
          (Rendering|Components|Sprite|SetSprite (Variables|/Game/MainGameContent/MemoryBP/Blueprints/BP_MemoryCard.BP_MemoryCard_C|GetSprite _returnvalue) _output_get_4)
          (Utilities|Array|RemoveIndex (Variables|Default|GetCardsSpawnPoolCache) _output_get_3) ; DO NOT USE "REMOVE ITEM"\n(That would remove ALL instances\nof said item, deleting the duplicate\nMemoryCard too!)
          ;;[1 1 1] Refill "CardsSpawnPool" only when its Empty
          (if (== (Utilities|Array|Length _cardsspawnpool_2) 0)
            (for _array_element_3 (Utilities|Struct|BreakFrontSpriteStruct (Variables|Default|GetFrontSpriteStruct))
              (Utilities|Array|AddUnique _cardsspawnpool_2 _array_element_3))))))
    (:then_1
      ;[1 1 1] Create UMG
      (bind _returnvalue_2 (UserInterface|CreateWidget "/Game/MainGameContent/MemoryBP/Blueprints/UMG/UI_ScoreBanner.UI_ScoreBanner_C"))
      (bind _output_get_5 (Variables|Default|SetScoreBannerRef _returnvalue_2))
      (UserInterface|Viewport|AddtoViewport _output_get_5 0))))

(event Input|KeyboardEvents|Delete
  (params (Key :type Key%20Structure :default "None"))
  ;[0 0.5572 1] SaveLogic
  (:Pressed
    ;;[1 1 1] Delete Savegame
    (Development|PrintString "SAVEGAME DELTED")
    (SaveGame|DeleteGameinSlot "FirstSlot")))

(fn ConstructionScript
  ;[1 1 1] Create Spawn Points for the Cards to use later (Event Graph)
  (bind _poly_center (Utilities|2DGridExecutionMacro (Variables|MemorySettings|GetCardSpacing) (Transformation|GetActorLocation self) 10 7)
    (:Per%20Poly%20Execution
      (Utilities|Array|Add (Variables|Default|GetSpawnSlots) _poly_center))))